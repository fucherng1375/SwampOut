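; Fluid Flux simulation modifier actor that wraps a BPFluxModifierWaveComponent for wave effects.
; Construction runs the parent script, then adds a box component snapped to the wave component's location, rotation and scale.
; It exposes the component's material instance as its only wave texture material, while CanRenderWave always returns false.
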(fn `CanRenderWave`
  (returns (CanRender :type Boolean))
  (return false))

(fn `GetWaveTextureMaterials`
  (returns (MaterialInstances :type "Array of MaterialInstanceDynamic Object Reference"))
  (return (`|MakeArray` (`/Game/Assets/Chernobyl_Theme/Landscape/Ocean/FluidFlux/Simulation/Modifiers/Components/BP_FluxModifierWaveComponent.MaterialInstance` (`self.BP_FluxModifierWaveComponent`)))))

(fn `UserConstructionScript`
  (`parent.UserConstructionScript`)
  (bind _returnvalue (`AddComponent|NODE_AddBoxComponent-0` :`bManualAttachment` true))
  (`SceneComponent.K2_AttachToComponent` _returnvalue (`self.BP_FluxModifierWaveComponent`) "None" "SnapToTarget" "SnapToTarget" "SnapToTarget" true))