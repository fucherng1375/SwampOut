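; BP_FluxHeightMap is a Fluid Flux tool actor that captures a ground heightmap of the world through a FluxHeightMapComponent.
; InitCapture runs at construction and BeginPlay, passing capture area, tile limit, domain texture and scene visibility to the component, then initializing it with the capture component.
; It also sets up optional editor and in-game debug display using a debug mesh and volume.
; CaptureGroundHeightmap triggers the component's ground map generation.
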(event `self.ReceiveBeginPlay`
  (`self.InitCapture`))

(fn `CaptureGroundHeightmap`
  (`/Game/Assets/Chernobyl_Theme/Landscape/Ocean/FluidFlux/Tools/Heightmap/Blueprints/BP_FluxHeightMapComponent.GenerateGroundMap` (`self.FluxHeightMapComponent`) false))

(fn `InitCapture`
  (`/Game/Assets/Chernobyl_Theme/Landscape/Ocean/FluidFlux/Tools/Heightmap/Blueprints/BP_FluxHeightMapComponent.SetConfig` (`self.FluxHeightMapComponent`) (`self.CaptureWorldHeight`) (`self.CaptureWorldPixelSize`) (* (`self.CaptureWorldLimitTileSize(M)`) 100) (`self.DomainTexture`) (`self.SceneVisibility`) 0.0)
  (`/Game/Assets/Chernobyl_Theme/Landscape/Ocean/FluidFlux/Tools/Heightmap/Blueprints/BP_FluxHeightMapComponent.InitializeAll` (`self.FluxHeightMapComponent`) (`self.CaptureComponent`))
  (`/Game/Assets/Chernobyl_Theme/Landscape/Ocean/FluidFlux/Tools/Heightmap/Blueprints/BP_FluxHeightMapComponent.InitlializeDebug` (`self.FluxHeightMapComponent`) (`self.Debug`) (`self.CaptureDebugInEditor`) (`self.CaptureDebugInGame`) (`self.Volume`)))

(fn `UserConstructionScript`
  (`self.InitCapture`))