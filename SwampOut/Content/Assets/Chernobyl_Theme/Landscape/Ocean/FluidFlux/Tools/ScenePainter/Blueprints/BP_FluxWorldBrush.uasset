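; FluidFlux world brush actor that paints a value into scene painters as a rectangle with adjustable roundness and hardness.
; Construction resizes the preview, asks every BPI_FluxWorldPainter actor to re-render, and feeds shape and value to the preview through custom primitive data.
; Draw runs only for a matching canvas type, setting material parameters and drawing at the actor transform.
; Brush color alpha encodes the inverse of additive blend.
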(fn `Draw`
  (params (Material :type "MaterialInstanceDynamic Object Reference (by ref)") (Painter :type "/Game/Assets/Chernobyl_Theme/Landscape/Ocean/FluidFlux/Tools/ScenePainter/Blueprints/BP_FluxWorldPainterComponent Object Reference (by ref)"))
  (bind _targetvalue (`self.TargetValue`))
  (if (== (`/Game/Assets/Chernobyl_Theme/Landscape/Ocean/FluidFlux/Tools/ScenePainter/Blueprints/BP_FluxWorldPainterComponent.CanvasType` Painter) (`self.Canvas`))
    (`MaterialInstanceDynamic.SetScalarParameterValue` (`local.Material`) "Hardness" (`self.ShapeHardness`))
    (`MaterialInstanceDynamic.SetScalarParameterValue` (`local.Material`) "Radius" (`self.ShapeRoundness`))
    (`MaterialInstanceDynamic.SetVectorParameterValue` (`local.Material`) "BrushColor" (`KismetMathLibrary.MakeColor` _targetvalue _targetvalue _targetvalue (- 1.0 (`self.BlendAdditive`))))
    (`/Game/Assets/Chernobyl_Theme/Landscape/Ocean/FluidFlux/Tools/ScenePainter/Blueprints/BP_FluxWorldPainterComponent.DrawRect` (`local.Painter`) (`local.Material`) (`self.GetTransform`))))

(fn `UserConstructionScript`
  (`SceneComponent.K2_SetRelativeTransform` (`self.Preview`) (`KismetMathLibrary.MakeTransform` (0.0 0.0 0.0) (struct) (0.01 0.01 1.0)) false false)
  (bind _outactors (`GameplayStatics.GetAllActorsWithInterface` "/Game/Assets/Chernobyl_Theme/Landscape/Ocean/FluidFlux/Tools/ScenePainter/Blueprints/BPI_FluxWorldPainter.BPI_FluxWorldPainter_C"))
  (for _array_element _outactors
    (message `/Game/Assets/Chernobyl_Theme/Landscape/Ocean/FluidFlux/Tools/ScenePainter/Blueprints/BPI_FluxWorldPainter.RenderScenePainter` _array_element)
    ;[1 1 1] Debug
    (`/Engine/EditorBlueprintResources/StandardMacros.IsValid` (`self.Preview`)
      (:`Is Valid`
        (`PrimitiveComponent.SetCustomPrimitiveDataFloat` (`self.Preview`) 0 (`self.ShapeRoundness`))
        (`PrimitiveComponent.SetCustomPrimitiveDataFloat` (`self.Preview`) 1 (`self.ShapeHardness`))
        (`PrimitiveComponent.SetCustomPrimitiveDataFloat` (`self.Preview`) 2 (`self.TargetValue`))))))