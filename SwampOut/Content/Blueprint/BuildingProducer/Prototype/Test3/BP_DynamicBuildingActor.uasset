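; Prototype generated dynamic mesh actor that builds a procedural wall box using Geometry Script.
; On rebuild it sizes and offsets the box from the Position vector, then scales UVs with wall length, clamped to a minimum, and prints that scale.
; A separate MeshGenerator function, not called within this Blueprint, boolean-subtracts a cutter box from a wall and bakes the result and its collision to a static mesh asset.
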(event `self.OnRebuildGeneratedMesh`
  (params (TargetMesh :type "DynamicMesh Object Reference"))
  (bind _position_x (`KismetMathLibrary.BreakVector` (`self.Position`)))
  (bind (_position_x_2 _position_y _position_z) (`KismetMathLibrary.BreakVector` (`self.Position`)))
  (bind _position_x_3 (`KismetMathLibrary.BreakVector` (`self.Position`)))
  (bind _returnvalue (`KismetMathLibrary.FMax` (* (`self.UVSizePerWall`) (/ _position_x 250.0)) (`self.UVSizePerWall`)))
  (bind _returnvalue_2 (`GeometryScriptLibrary_MeshPrimitiveFunctions.AppendBox` TargetMesh (struct) (`KismetMathLibrary.MakeTransform` (`KismetMathLibrary.MakeVector` (/ _position_x_2 2.0) _position_y _position_z) (`self.Transform Rotation`)) _position_x_3 10.0 250.0 3 0 0 "Base" null))
  (`GeometryScriptLibrary_MeshUVFunctions.ScaleMeshUVs` _returnvalue_2 0 (`KismetMathLibrary.Conv_DoubleToVector2D` _returnvalue) (0.0 0.0) (struct) null)
  (`KismetSystemLibrary.PrintString` (`KismetStringLibrary.Conv_DoubleToString` _returnvalue)))

(fn `MeshGenerator`
  (params (TargetMesh :type "DynamicMesh Object Reference") (Dimension :type "Vector Structure" :default (100.0 100.0 100.0)) (ToStaticMeshAsset :type "StaticMesh Object Reference"))
  (locals (Cuter :type "DynamicMesh Object Reference"))
  (bind (_dimension_x _dimension_y _dimension_z) (`KismetMathLibrary.BreakVector` (`local.Dimension`)))
  (bind _tostaticmeshasset (`local.ToStaticMeshAsset`))
  (`|ExecutionSequence`
    (:`then_0`
      (bind _returnvalue (`self.AllocateComputeMesh`))
      (bind _returnvalue_2 (`GeometryScriptLibrary_MeshPrimitiveFunctions.AppendBox` _returnvalue (struct) (struct) _dimension_x _dimension_y _dimension_z 0 0 0 "Base" null))
      (set `local.Cuter` _returnvalue_2))
    (:`then_1`
      (bind _returnvalue_3 (`GeometryScriptLibrary_MeshPrimitiveFunctions.AppendBox` TargetMesh (struct) (struct) 100.0 10.0 250.0 0 0 0 "Base" null))
      (bind _returnvalue_4 (`GeometryScriptLibrary_MeshBooleanFunctions.ApplyMeshBoolean` _returnvalue_3 (struct) (`local.Cuter`) (`KismetMathLibrary.Conv_VectorToTransform` (`self.Position`)) "Subtract" (struct) null))
      (bind _returnvalue_5 (`GeometryScriptLibrary_StaticMeshFunctions.CopyMeshToStaticMesh` _returnvalue_4 _tostaticmeshasset (struct) (struct) null)
        (:`Success`
          (`GeometryScriptLibrary_CollisionFunctions.SetStaticMeshCollisionFromMesh` _returnvalue_5 _tostaticmeshasset (struct) (struct :`bMarkAsCustomized` true) null))))))

(fn `UserConstructionScript`)