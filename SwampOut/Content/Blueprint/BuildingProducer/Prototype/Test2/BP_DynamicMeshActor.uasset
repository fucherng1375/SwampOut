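; Prototype generated dynamic mesh actor that builds a thin box panel with a box-shaped hole cut out, using Geometry Script.
; On rebuild, MeshGenerator creates a cutter box in a compute mesh, appends the panel to the target mesh, then boolean-subtracts the cutter at the BooleanCut transform.
; It then attempts a copy to a static mesh asset and sets collision on success, though the rebuild event passes no asset.
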(event `self.OnRebuildGeneratedMesh`
  (params (TargetMesh :type "DynamicMesh Object Reference"))
  (`self.MeshGenerator` TargetMesh (100.0 100.0 200.0)))

(fn `MeshGenerator`
  (params (TargetMesh :type "DynamicMesh Object Reference") (Dimension :type "Vector Structure" :default (100.0 100.0 100.0)) (ToStaticMeshAsset :type "StaticMesh Object Reference"))
  (locals (Cuter :type "DynamicMesh Object Reference"))
  (bind (_dimension_x _dimension_y _dimension_z) (`KismetMathLibrary.BreakVector` (`local.Dimension`)))
  (bind _tostaticmeshasset (`local.ToStaticMeshAsset`))
  (`|ExecutionSequence`
    (:`then_0`
      (bind _returnvalue (`self.AllocateComputeMesh`))
      (bind _returnvalue_2 (`GeometryScriptLibrary_MeshPrimitiveFunctions.AppendBox` _returnvalue (struct) (struct) _dimension_x _dimension_y _dimension_z 0 0 0 "Base" null))
      (set `local.Cuter` _returnvalue_2))
    (:`then_1`
      (bind _returnvalue_3 (`GeometryScriptLibrary_MeshPrimitiveFunctions.AppendBox` TargetMesh (struct) (struct) 100.0 10.0 250.0 0 0 0 "Base" null))
      (bind _returnvalue_4 (`GeometryScriptLibrary_MeshBooleanFunctions.ApplyMeshBoolean` _returnvalue_3 (struct) (`local.Cuter`) (`KismetMathLibrary.Conv_VectorToTransform` (`self.BooleanCut`)) "Subtract" (struct) null))
      (bind _returnvalue_5 (`GeometryScriptLibrary_StaticMeshFunctions.CopyMeshToStaticMesh` _returnvalue_4 _tostaticmeshasset (struct) (struct) null)
        (:`Success`
          (`GeometryScriptLibrary_CollisionFunctions.SetStaticMeshCollisionFromMesh` _returnvalue_5 _tostaticmeshasset (struct) (struct :`bMarkAsCustomized` true) null))))))

(fn `UserConstructionScript`)